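; BP_Intel is an interactable intel object that the first-person character can use, which removes it from the world.
; A collision sphere adds the actor to the FirstPersonCharacter's InteractableObjects list on overlap begin and removes it on overlap end.
; The UseInteractableObject event simply destroys the actor, with no other pickup logic in this Blueprint.
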(event `self.Sphere_Collision.OnComponentBeginOverlap`
  (params (OverlappedComponent :type "PrimitiveComponent Object Reference") (OtherActor :type "Actor Object Reference") (OtherComp :type "PrimitiveComponent Object Reference") (OtherBodyIndex :type Integer) (bFromSweep :type Boolean) (SweepResult :type "HitResult Structure (by ref)"))
  (bind _asfirst_person_character (cast `/Game/FirstPersonBP/Blueprints/FirstPersonCharacter` OtherActor))
  (`KismetArrayLibrary.Array_Add` (`/Game/FirstPersonBP/Blueprints/FirstPersonCharacter.InteractableObjects` _asfirst_person_character) self))

(event `self.Sphere_Collision.OnComponentEndOverlap`
  (params (OverlappedComponent :type "PrimitiveComponent Object Reference") (OtherActor :type "Actor Object Reference") (OtherComp :type "PrimitiveComponent Object Reference") (OtherBodyIndex :type Integer))
  (bind _asfirst_person_character (cast `/Game/FirstPersonBP/Blueprints/FirstPersonCharacter` OtherActor))
  (`KismetArrayLibrary.Array_RemoveItem` (`/Game/FirstPersonBP/Blueprints/FirstPersonCharacter.InteractableObjects` _asfirst_person_character) self))

(event `/Game/MyProjectNew/FrameWork/BP_TrueInterface.UseInteractableObject`
  (`self.K2_DestroyActor`))

(fn `UserConstructionScript`)